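; Player-controlled tank pawn with turret aiming, firing and self-destruction.
; Input drives a TankMovement component (drive, turn, sprint, brake, jump), turret yaw, clamped spring-arm and barrel pitch, and Launcher firing.
; A Delay in Tick increments BulletCount every two seconds and feeds the deprojected crosshair direction to BarrelOrientingMovement.
; Projectile hits or SelfDestruct hide the body, disable input, detach the camera arm and destructible, then fracture it with radial damage.
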(event EventTick
  (params (DeltaSeconds :type Float%20%28single-precision%29))
  ;[1 1 1] Tick
  (Utilities|FlowControl|Delay 2.0)
  (Math|Integer|IncrementInt (Variables|Default|GetBulletCount)
    (:%20%20
      (Variables|/Script/TT3D.OrientingMovementComponent|SetDirection (Variables|Default|GetBarrelOrientingMovement) (- (.WorldPosition (Class|GameplayStatics|DeprojectScreentoWorld (Game|GetPlayerController 0) (Class|CanvasPanelSlot|GetPosition (Class|WidgetLayoutLibrary|SlotasCanvasSlot (Variables|Default|GetCrosshair))))) (Transformation|GetWorldLocation (Variables|Default|GetCamera)))))))

(event EventBeginPlay
  ;[1 1 1] Begin
  (bind _returnvalue (UserInterface|CreateWidget "/Game/Blueprints/Crosshair.Crosshair_C"))
  (UserInterface|Viewport|AddtoViewport _returnvalue 0)
  (Variables|Default|SetCrosshair (Variables|/Game/Blueprints/Crosshair.Crosshair_C|GetImage_61 _returnvalue))
  (Collision|SetCollisionEnabled (Variables|Default|GetDestructible) "NoCollision")
  (Components|Movement|SetUpdatedComponent (Variables|Default|GetTankMovement) (Variables|Default|GetBody))
  (Components|Movement|SetUpdatedComponent (Variables|Default|GetBarrelOrientingMovement) (Variables|Default|GetBarrel)))

(event Collision|EventHit
  (params (MyComp :type Primitive%20Component%20Object%20Reference) (Other :type Actor%20Object%20Reference) (OtherComp :type Primitive%20Component%20Object%20Reference) (bSelfMoved :type Boolean) (HitLocation :type Vector :default "0, 0, 0") (HitNormal :type Vector :default "0, 0, 0") (NormalImpulse :type Vector :default "0, 0, 0") (Hit :type Hit%20Result%20Structure%20%28by%20ref%29))
  (bind _destructible (Variables|Default|GetDestructible))
  ;[1 1 1] Destruction
  (Utilities|Casting|CastToBP_Projectile Other)
  (Rendering|SetVisibility (Variables|Default|GetBody) false false)
  (Input|DisableInput 0)
  (Transformation|DetachFromComponent (Variables|Default|GetSpringArm) "KeepWorld" "KeepWorld" "KeepWorld" true)
  (Class|DestructibleComponent|ApplyRadiusDamage _destructible 1.0 (Transformation|GetWorldLocation _destructible) 1e+02 0.0 false))

(event Input|ActionEvents|InputActionJump
  (params (Key :type Key%20Structure))
  ;[1 1 1] Movement
  (:Pressed
    (Class|TankMovementComponent|Jump (Variables|Default|GetTankMovement))))

(event Input|ActionEvents|InputActionFire
  (params (Key :type Key%20Structure))
  ;[1 1 1] Fire
  (:Pressed
    (Class|Launcher|Fire (Variables|Default|GetLauncher))))

(event Input|ActionEvents|InputActionSelfDestruct
  (params (Key :type Key%20Structure))
  (bind _destructible (Variables|Default|GetDestructible))
  ;[1 1 1] Destruction
  (:Pressed
    (Rendering|SetVisibility (Variables|Default|GetBody) false false)
    (Input|DisableInput 0)
    (Transformation|DetachFromComponent (Variables|Default|GetSpringArm) "KeepWorld" "KeepWorld" "KeepWorld" true)
    (Class|DestructibleComponent|ApplyRadiusDamage _destructible 1.0 (Transformation|GetWorldLocation _destructible) 1e+02 0.0 false)))

(event Input|ActionEvents|InputActionBreak
  (params (Key :type Key%20Structure))
  (bind _tankmovement (Variables|Default|GetTankMovement))
  ;[1 1 1] Movement
  (:Pressed
    (Class|TankMovementComponent|Break _tankmovement))
  (:Released
    (Class|TankMovementComponent|UnBreak _tankmovement)))

(event Input|ActionEvents|InputActionSprint
  (params (Key :type Key%20Structure))
  (bind _tankmovement (Variables|Default|GetTankMovement))
  ;[1 1 1] Movement
  (:Pressed
    (Class|TankMovementComponent|Sprint _tankmovement))
  (:Released
    (Class|TankMovementComponent|UnSprint _tankmovement)))

(event Input|AxisEvents|InputAxisMoveForward
  (params (AxisValue :type Float%20%28single-precision%29))
  ;[1 1 1] Movement
  (Class|TankMovementComponent|MoveForward (Variables|Default|GetTankMovement) AxisValue))

(event Input|AxisEvents|InputAxisTurn
  (params (AxisValue :type Float%20%28single-precision%29))
  ;[1 1 1] Aiming
  (Transformation|AddRelativeRotation (Variables|Default|GetTurret) (Math|Rotator|MakeRotator 0.0 0.0 (* AxisValue (Utilities|Time|GetTimeSeconds) 0.3)) false false))

(event Input|AxisEvents|InputAxisLookUp
  (params (AxisValue :type Float%20%28single-precision%29))
  (bind _springarm (Variables|Default|GetSpringArm))
  (bind _relativerotation (Variables|/Script/Engine.SceneComponent|GetRelativeRotation _springarm))
  (bind (_roll _pitch _yaw) (Math|Rotator|BreakRotator _relativerotation))
  ;[1 1 1] Aiming
  (bind _output_get (Variables|Default|SetPitch (Math|Float|Clamp(Float) (+ (Variables|Default|GetPitch) (* (Utilities|Time|GetTimeSeconds) AxisValue 0.5)) -2e+01 4e+01)))
  (Transformation|SetRelativeRotation _springarm (Math|Rotator|MakeRotator _roll (* _output_get -1.0) _yaw) false false)
  (Transformation|SetRelativeRotation (Variables|Default|GetBarrel) (Math|Rotator|MakeRotator (+ _output_get -3e+01) 0.0 0.0) false false))

(event Input|AxisEvents|InputAxisMoveRight
  (params (AxisValue :type Float%20%28single-precision%29))
  ;[1 1 1] Movement
  (Class|TankMovementComponent|Turn (Variables|Default|GetTankMovement) AxisValue))

(fn ConstructionScript)